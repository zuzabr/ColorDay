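; Base melee attack ability for NPCs that damages a player overlapping the NPC.
; On activation it takes the first valid overlapping BP_Player, sends a Shared.Damage gameplay event, applies damage and ends immediately.
; HandleApplyDamage builds an enemy damage spec from GE_SharedDealDamage and ScalableDamage and applies it to the payload's target.
; The event and damage calls run even when no player is found, leaving the target empty.
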(event `self.K2_ActivateAbility`
  (bind _gameplayeventdata (make `GameplayEventData` (struct :`TagName` "Shared.Damage") (`self.GetNPC`) (`self.Player`)))
  ;[0.5677 0 0.009004 0.5] Make a melee logic for attack in NPC in C++
  (set `self.Player` null)
  (for _array_element (`Actor.GetOverlappingActors` (`self.GetNPC`) "/Game/ColorDay/Blueprints/Player/BP_Player.BP_Player_C")
    (`/Engine/EditorBlueprintResources/StandardMacros.IsValid` _array_element
      (:`Is Valid`
        (set `self.Player` _array_element)
        (break))))
  (`AbilitySystemBlueprintLibrary.SendGameplayEventToActor` null (struct :`TagName` "Shared.Damage") _gameplayeventdata)
  (`self.HandleApplyDamage` _gameplayeventdata)
  (`self.K2_EndAbility`))

(fn `HandleApplyDamage`
  (params (Payload :type "GameplayEventData Structure"))
  (`ColorDayFunctionLibrary.ApplyGameplayEffectSpecHandleToTargetActor` Payload_Instigator Payload_Target (`self.MakeEnemyDamageEffectSpecHandle` "/Game/ColorDay/Blueprints/GameplayEffects/GE_SharedDealDamage.GE_SharedDealDamage_C" (`self.Scalable Damage`) (struct :`TagName` "Shared.Damage"))))